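; BP_Item is a pickup item actor for the inventory system.
; On BeginPlay it applies its Material to a Sphere component.
; Pick Up Item prints a debug message, calls DestroyItem and returns the Item variable.
; DestroyItem waits briefly before destroying the actor.
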(event Custom|Destroy%20Item
  (Utilities|FlowControl|Delay 0.1)
  (Actor|DestroyActor))

(event EventBeginPlay
  (Rendering|Material|SetMaterial (Variables|Default|GetSphere) 0 (Variables|Default|Getmaterial)))

(fn ConstructionScript)

(fn PickUpItem
  (Development|PrintString "item picked")
  (CallFunction|DestroyItem)
  (return (Variables|Default|Getitem)))